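; Player avatar Blueprint that drives its visual effects, level-end widgets and pause toggle.
; Timelines animate moving to an entrance, portal morphing, stopping momentum and two deaths: a shrink into a black hole or a cylinder burst with camera shake.
; Display events create tutorial or regular transition screens and the win screen.
; Pausing flip-flops a widget and freezes the avatar through high linear damping instead of pausing the game.
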(event EventBeginPlay
  (Input|EnableInput (Game|GetPlayerController 0)))

(event Collision|EventActorBeginOverlap
  (params (OtherActor :type Actor%20Object%20Reference)))

(event EventPauseGame
  (bind _collision (Variables|Default|GetCollision))
  (if (not (Variables|Default|GetbIsInLevelStart))
    (Utilities|FlowControl|FlipFlop
      (:A
        (Variables|Default|SetbGameIsPaused true)
        (bind _returnvalue (UserInterface|CreateWidget "/Game/Blueprints/UI/BP_Pause.BP_Pause_C"))
        (Variables|Default|SetPauseWidget _returnvalue)
        (UserInterface|Viewport|AddtoViewport _returnvalue 0)
        (Class|PrimitiveComponent|SetLinearDamping _collision 1e+03))
      (:B
        (Variables|Default|SetbGameIsPaused false)
        (Widget|RemovefromParent (Variables|Default|GetPauseWidget))
        (Class|PrimitiveComponent|SetLinearDamping _collision 0.0)))))

(event EventTick
  (params (DeltaSeconds :type Float%20%28single-precision%29)))

(event EventTLMovetoEntrance
  (bind _movetoentrance (Timeline|MoveToEntrance PlayFromStart)
    (:Update
      (Class|Avatar|MovetoEntrance _movetoentrance))
    (:Finished
      (Class|Avatar|AfterMove))))

(event EventTLDeathEffect
  (params (bDeathByBlackHole :type Boolean) (DeathLocation :type Vector :default "0, 0, 0") (BlackHoleLocation :type Vector :default "0, 0, 0"))
  (bind _deathcylinder (Variables|Default|GetDeathCylinder))
  (if bDeathByBlackHole
    (Audio|PlaySound2D "/Game/Sound/DeathByBlackHole.DeathByBlackHole" 1.0 1.0 0.0 0 0)
    (bind _newtrack_0 (Timeline|TL_ShrinkSpheroid PlayFromStart)
      (:Update
        (Transformation|SetRelativeScale3D (Variables|Default|GetPlaneMesh) (Math|Vector|Lerp(Vector) (Variables|Default|GetPortalMorphBig) (Variables|Default|GetPortalMorphSmall) _newtrack_0))
        (Transformation|SetActorLocation (Math|Vector|Lerp(Vector) (Math|Vector|MakeVector 454.912842 (.y DeathLocation) (.z DeathLocation)) (Math|Vector|MakeVector 454.912842 (.y BlackHoleLocation) (.z BlackHoleLocation)) _newtrack_0) false false))
      (:Finished
        (Class|Avatar|AfterBlackHoleShrink)))
    (else
      (Class|SpheroidXGameModeBase|PlayCameraShake (Variables|Default|GetGameModeRef) "Death")
      (Audio|PlaySound2D "/Game/Sound/Death.Death" 1.0 1.0 0.0 0 0)
      (Development|SetHiddeninGame (Variables|Default|GetDeathCylinder) false false)
      (bind (_direction _scale _cylinder) (Timeline|DeathEffect PlayFromStart)
        (:Update
          (Class|Avatar|DeathEffect _scale)
          (Transformation|SetRelativeScale3D (Variables|Default|GetDeathCylinder) (Math|Vector|Lerp(Vector) "0, 0,2.000000" (Variables|Default|GetDeathCylinderBig) _cylinder)))
        (:Finished
          (Class|Avatar|EffectCleanUp)
          (Transformation|SetRelativeScale3D _deathcylinder "0, 0,2.000000")
          (Development|SetHiddeninGame _deathcylinder true false))))))

(event EventTLBoostEffect
  (bind _boostplane (Variables|Default|GetBoostPlane))
  (Development|SetHiddeninGame _boostplane false false)
  (Utilities|FlowControl|Delay 0.1)
  (Development|SetHiddeninGame _boostplane true false))

(event EventTLStopMomentumEffect
  (bind _scale (Timeline|StopMomentum PlayFromStart)
    (:Update
      (Class|Avatar|StopMomentumEffect _scale))))

(event EventDisplayTime
  (if (Variables|Default|GetbIsTutorialLevel)
    (Viewport|RemoveAllWidgets)
    (bind _returnvalue (UserInterface|CreateWidget "/Game/Blueprints/UI/LevelTransitionsBasicTraining.LevelTransitionsBasicTraining_C"))
    (UserInterface|Viewport|AddtoViewport _returnvalue 0)
    (else
      (Viewport|RemoveAllWidgets)
      (bind _returnvalue_2 (UserInterface|CreateWidget "/Game/Blueprints/UI/LevelTransitionsWidget.LevelTransitionsWidget_C"))
      (UserInterface|Viewport|AddtoViewport _returnvalue_2 0)
      (Variables|/Game/Blueprints/UI/LevelTransitionsWidget.LevelTransitionsWidget_C|SetPreviousLevel _returnvalue_2 (Variables|Default|GetPreviousLevel))
      (Variables|/Game/Blueprints/UI/LevelTransitionsWidget.LevelTransitionsWidget_C|SetCurrentLevel _returnvalue_2 (Variables|Default|GetCurrentLevel))
      (Variables|/Game/Blueprints/UI/LevelTransitionsWidget.LevelTransitionsWidget_C|SetNextLevel _returnvalue_2 (Variables|Default|GetNextLevel))
      (if (Variables|Default|GetbIsFirstLevel)
        (Default|RemoveButtonPreviousLevel _returnvalue_2)))))

(event EventPortalMorph
  (bind _morphscale (Timeline|TL_PortalMorph PlayFromStart)
    (:Update
      (Transformation|SetRelativeScale3D (Variables|Default|GetPlaneMesh) (Math|Vector|Lerp(Vector) (Variables|Default|GetPortalMorphBig) (Variables|Default|GetPortalMorphSmall) _morphscale)))
    (:Finished
      (Class|Avatar|PortalMorphCleanUp))))

(event EventCreateWinScreen
  (bind _returnvalue (UserInterface|CreateWidget "/Game/Blueprints/UI/Congratulations.Congratulations_C"))
  (UserInterface|Viewport|AddtoViewport _returnvalue 0))

(fn ConstructionScript)