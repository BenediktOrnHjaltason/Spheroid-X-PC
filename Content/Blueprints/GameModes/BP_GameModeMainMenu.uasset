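; Main menu game mode that loads saved level times and picks the opening screen on BeginPlay.
; It hides the mouse cursor, enables input and, when UnlockAllLevels is set, overwrites every entry in the game instance's LevelsLocked array.
; The game instance's LevelIndex selects the widget: a sentinel value shows the main menu, otherwise the matching six-level page of eight level-select screens appears, followed by the menu sound.
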(event EventBeginPlay
  (Variables|/Script/Engine.PlayerController|SetbShowMouseCursor (Game|GetPlayerController 0) false)
  (bind _asbp_game_instance (Utilities|Casting|CastToBP_GameInstance (Game|GetGameInstance)))
  (bind _output_get (Variables|Default|SetGameInstanceRef _asbp_game_instance))
  ;[1 1 1] Loads all game state
  (Class|SpheroidGameInstance|LoadLevelTimesfromDisk _output_get)
  (Input|EnableInput (Game|GetPlayerController 0) 0)
  (if (Variables|Default|GetbUnlockAllLevels)
    (for (_ _array_index) (Variables|/Script/SpheroidX.SpheroidGameInstance|GetLevelsLocked (Variables|Default|GetGameInstanceRef))
      (Utilities|Array|SetArrayElem (Variables|/Script/SpheroidX.SpheroidGameInstance|GetLevelsLocked (Variables|Default|GetGameInstanceRef)) _array_index false)))
  (Math|Integer|CompareInt (Variables|/Script/SpheroidX.SpheroidGameInstance|GetLevelIndex (Variables|Default|GetGameInstanceRef)) 99
    (:==
      (bind _returnvalue (UserInterface|CreateWidget "/Game/Blueprints/UI/MainMenuWidget.MainMenuWidget_C"))
      (UserInterface|Viewport|AddtoViewport _returnvalue 0)
      (Variables|Default|SetMainMenuWidget _returnvalue)
      (Audio|PlaySound2D "/Game/Sound/MainMenuCue.MainMenuCue" 1.0 1.0 0.0 0 0 :!label _label))
    (:<
      (if (Math|Integer|InRange(Integer) (Variables|/Script/SpheroidX.SpheroidGameInstance|GetLevelIndex (Variables|Default|GetGameInstanceRef)) 0 5)
        (bind _returnvalue_2 (UserInterface|CreateWidget "/Game/Blueprints/UI/Levels1.Levels1_C"))
        (UserInterface|Viewport|AddtoViewport _returnvalue_2 0)
        (goto _label)
        (elif (Math|Integer|InRange(Integer) (Variables|/Script/SpheroidX.SpheroidGameInstance|GetLevelIndex (Variables|Default|GetGameInstanceRef)) 6 11)
          (bind _returnvalue_3 (UserInterface|CreateWidget "/Game/Blueprints/UI/Levels2.Levels2_C"))
          (UserInterface|Viewport|AddtoViewport _returnvalue_3 0)
          (goto _label)
          (elif (Math|Integer|InRange(Integer) (Variables|/Script/SpheroidX.SpheroidGameInstance|GetLevelIndex (Variables|Default|GetGameInstanceRef)) 12 17)
            (bind _returnvalue_4 (UserInterface|CreateWidget "/Game/Blueprints/UI/Levels3.Levels3_C"))
            (UserInterface|Viewport|AddtoViewport _returnvalue_4 0)
            (goto _label)
            (elif (Math|Integer|InRange(Integer) (Variables|/Script/SpheroidX.SpheroidGameInstance|GetLevelIndex (Variables|Default|GetGameInstanceRef)) 18 23)
              (bind _returnvalue_5 (UserInterface|CreateWidget "/Game/Blueprints/UI/Levels4.Levels4_C"))
              (UserInterface|Viewport|AddtoViewport _returnvalue_5 0)
              (goto _label)
              (elif (Math|Integer|InRange(Integer) (Variables|/Script/SpheroidX.SpheroidGameInstance|GetLevelIndex (Variables|Default|GetGameInstanceRef)) 24 29)
                (bind _returnvalue_6 (UserInterface|CreateWidget "/Game/Blueprints/UI/Levels5.Levels5_C"))
                (UserInterface|Viewport|AddtoViewport _returnvalue_6 0)
                (goto _label)
                (elif (Math|Integer|InRange(Integer) (Variables|/Script/SpheroidX.SpheroidGameInstance|GetLevelIndex (Variables|Default|GetGameInstanceRef)) 30 35)
                  (bind _returnvalue_7 (UserInterface|CreateWidget "/Game/Blueprints/UI/Levels6.Levels6_C"))
                  (UserInterface|Viewport|AddtoViewport _returnvalue_7 0)
                  (goto _label)
                  (elif (Math|Integer|InRange(Integer) (Variables|/Script/SpheroidX.SpheroidGameInstance|GetLevelIndex (Variables|Default|GetGameInstanceRef)) 36 41)
                    (bind _returnvalue_8 (UserInterface|CreateWidget "/Game/Blueprints/UI/Levels7.Levels7_C"))
                    (UserInterface|Viewport|AddtoViewport _returnvalue_8 0)
                    (goto _label)
                    (elif (Math|Integer|InRange(Integer) (Variables|/Script/SpheroidX.SpheroidGameInstance|GetLevelIndex (Variables|Default|GetGameInstanceRef)) 42 47)
                      (bind _returnvalue_9 (UserInterface|CreateWidget "/Game/Blueprints/UI/Levels8.Levels8_C"))
                      (UserInterface|Viewport|AddtoViewport _returnvalue_9 0)
                      (goto _label))))))))))))

(event EventTick
  (params (DeltaSeconds :type Float%20%28single-precision%29)))

(fn ConstructionScript)