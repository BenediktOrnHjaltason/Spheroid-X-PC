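; Game mode that shows the mouse cursor, starts a level sound cue and relays gameplay feedback to the main HUD and camera.
; HUD events map an animation type to countdown, goal, respawn or fade animations, and update the portal button icon, optionally flagging a death reset.
; A camera shake event plays a death world shake at the Spheroid's camera location when the Spheroid is valid.
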(event EventBeginPlay
  (Variables|/Script/Engine.PlayerController|SetbShowMouseCursor (Game|GetPlayerController 0) true)
  (Audio|PlaySound2D "/Game/Sound/LevelSoundCue.LevelSoundCue" 1.0 1.0 0.0 0 0))

(event EventTick
  (params (DeltaSeconds :type Float%20%28single-precision%29)))

(event EventPlayHUDAnimation
  (params (Animation :type EHUDAnimations%20Enum :default "CountDown"))
  (bind _mainhudref (Variables|Default|GetMainHudRef))
  (switch Utilities|FlowControl|Switch|SwitchonEHUDAnimations Animation
    (:CountDown
      (Default|AnimPlayCountDown _mainhudref))
    (:ReachedGoal
      (Default|AnimPlayGoalPhew _mainhudref))
    (:RespawnGo
      (Default|AnimPlayRespawnGo _mainhudref))
    (:FadeInOutRemaining
      (Default|AnimPlayFadeRemaining _mainhudref))))

(event EventChangePortalButtonIcon
  (params (bIsforDeathReset :type Boolean))
  (bind _mainhudref (Variables|Default|GetMainHudRef))
  (if bIsforDeathReset
    (Variables|/Game/Blueprints/UI/MainHUD.MainHUD_C|SetbIsForDeathReset _mainhudref true))
  (Default|ChangePortalButtonIcon _mainhudref))

(event EventPlayCameraShake
  (params (CameraShake :type ECameraShakes%20Enum :default "Death"))
  (bind _spheroid (Variables|Default|GetSpheroid))
  (if (Utilities|IsValid _spheroid)
    (switch Utilities|FlowControl|Switch|SwitchonECameraShakes CameraShake
      (:Death
        (Camera|PlayWorldCameraShake "/Game/CameraShake_Death.CameraShake_Death_C" (Transformation|GetWorldLocation (Variables|/Script/SpheroidX.Avatar|GetCamera _spheroid)) 5e+01 6e+01)))))

(fn ConstructionScript)