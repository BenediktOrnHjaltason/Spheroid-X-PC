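; Tutorial puzzle actor, StayStill, that starts when the bait key pickup is overlapped and opens a door if the player survives.
; Chained timelines push out the Confiner cylinder, then shrink it and its sphere collision in two steps, checking for death around pauses.
; StayStill_OnDeath flags failure, and a reset timeline retracts the confiner, restoring the key after a death.
; Tutorial game mode tracks active status and running state.
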(event Custom|StartPuzzle
  (Class|SpheroidXGameModeBase|StatusTurntoActive (Variables|Default|GetGameMode_Tutorial))
  (Variables|Default|SetbSequenceIsRunning true)
  (bind _pushoutcylinder (Timeline|PushOutCylinder PlayFromStart)
    (:Update
      (Transformation|SetRelativeLocation (Variables|Default|GetConfiner) (Math|Vector|Lerp(Vector) (Variables|Default|GetCylinderIn) (Variables|Default|GetCylinderOut) _pushoutcylinder) false false))
    (:Finished
      (if (Variables|Default|GetbSpheroidDied)
        (Variables|Default|SetSizeAtDeath (Variables|Default|GetCylinderSize3))
        (CallFunction|ResetPuzzle)
        (else
          (Utilities|FlowControl|Delay 2.0)
          (if (Variables|Default|GetbSpheroidDied)
            (Variables|Default|SetSizeAtDeath (Variables|Default|GetCylinderSize3))
            (CallFunction|ResetPuzzle)
            (else
              (bind _3_2 (Timeline|3%20to%202 PlayFromStart)
                (:Update
                  (Components|Sphere|SetSphereRadius (Variables|Default|GetSphereCollision) (Math|Float|Lerp (Variables|Default|GetCollisionRadius3) (Variables|Default|GetCollisionRadius2) _3_2) true)
                  (Transformation|SetRelativeScale3D (Variables|Default|GetConfiner) (Math|Vector|Lerp(Vector) (Variables|Default|GetCylinderSize3) (Variables|Default|GetCylinderSize2) _3_2)))
                (:Finished
                  (if (Variables|Default|GetbSpheroidDied)
                    (Variables|Default|SetSizeAtDeath (Variables|Default|GetCylinderSize2))
                    (CallFunction|ResetPuzzle)
                    (else
                      (Utilities|FlowControl|Delay 2.0)
                      (if (Variables|Default|GetbSpheroidDied)
                        (Variables|Default|SetSizeAtDeath (Variables|Default|GetCylinderSize2))
                        (CallFunction|ResetPuzzle)
                        (else
                          (bind _2_1 (Timeline|2%20to%201 PlayFromStart)
                            (:Update
                              (Components|Sphere|SetSphereRadius (Variables|Default|GetSphereCollision) (Math|Float|Lerp (Variables|Default|GetCollisionRadius2) (Variables|Default|GetCollisionRadius1) _2_1) true)
                              (Transformation|SetRelativeScale3D (Variables|Default|GetConfiner) (Math|Vector|Lerp(Vector) (Variables|Default|GetCylinderSize2) (Variables|Default|GetCylinderSize1) _2_1)))
                            (:Finished
                              (if (Variables|Default|GetbSpheroidDied)
                                (Variables|Default|SetSizeAtDeath (Variables|Default|GetCylinderSize1))
                                (CallFunction|ResetPuzzle)
                                (else
                                  (Utilities|FlowControl|Delay 2.0)
                                  (if (Variables|Default|GetbSpheroidDied)
                                    _
                                    (else
                                      (Variables|/Game/Blueprints/GameModes/BP_GameMode_Tutorial.BP_GameMode_Tutorial_C|SetbStayStillIsRunning (Variables|Default|GetGameMode_Tutorial) false)
                                      (Variables|Default|SetbSequenceIsRunning false)
                                      (CallFunction|OpenDoor)))
                                  (Variables|Default|SetSizeAtDeath (Variables|Default|GetCylinderSize1))
                                  (CallFunction|ResetPuzzle))))))))))))))))))

(event Custom|OnComponentBeginOverlap_Event_0
  (params (OverlappedComponent :type Primitive%20Component%20Object%20Reference) (OtherActor :type Actor%20Object%20Reference) (OtherComp :type Primitive%20Component%20Object%20Reference) (OtherBodyIndex :type Integer) (bFromSweep :type Boolean) (SweepResult :type Hit%20Result%20Structure%20%28by%20ref%29))
  (CallFunction|StartPuzzle))

(event Custom|ResetPuzzle
  (bind _confiner (Variables|Default|GetConfiner))
  (bind _baitkey (Variables|Default|GetBaitKey))
  (bind _childactor (Variables|/Script/Engine.ChildActorComponent|GetChildActor _baitkey))
  (Variables|/Game/Blueprints/GameModes/BP_GameMode_Tutorial.BP_GameMode_Tutorial_C|SetbStayStillIsRunning (Variables|Default|GetGameMode_Tutorial) true)
  (bind _2_1 (Timeline|Reset PlayFromStart)
    (:Update
      (Transformation|SetRelativeScale3D _confiner (Math|Vector|Lerp(Vector) (Variables|Default|GetSizeAtDeath) (Variables|Default|GetCylinderSize3) _2_1))
      (Transformation|SetRelativeLocation _confiner (Math|Vector|Lerp(Vector) (Variables|Default|GetCylinderOut) (Variables|Default|GetCylinderIn) _2_1) false false)
      (Components|Sphere|SetSphereRadius (Variables|Default|GetSphereCollision) (Math|Float|Lerp (Variables|Default|GetCollisionRadius1) (Variables|Default|GetCollisionRadius3) _2_1) true))
    (:Finished
      (Class|SpheroidXGameModeBase|StatusTurntoInactive (Variables|Default|GetGameMode_Tutorial))
      (if (Variables|Default|GetbSpheroidDied)
        (Collision|SetActorEnableCollision _childactor true)
        (Rendering|SetActorHiddenInGame _childactor false)
        (Variables|Default|SetbSpheroidDied false)))))

(event Custom|StayStill_OnDeath
  (if (Variables|/Game/Blueprints/GameModes/BP_GameMode_Tutorial.BP_GameMode_Tutorial_C|GetbStayStillIsRunning (Variables|Default|GetGameMode_Tutorial))
    (Variables|Default|SetbSpheroidDied true)
    (Utilities|FlowControl|Delay 2.0)))

(event Custom|OpenDoor
  (Utilities|FlowControl|Delay 2.0)
  (bind _newtrack_0 (Timeline|TL_OpenDoor PlayFromStart)
    (:Update
      (Transformation|SetRelativeLocation (Variables|Default|GetDoor) (Math|Vector|Lerp(Vector) "-26.193970,1.419556,604.231018" "-26.194397,-754.175171,604.231018" _newtrack_0) false false))))

(event EventBeginPlay
  (bind _asbp_game_mode_tutorial (Utilities|Casting|CastToBP_GameMode_Tutorial (Game|GetGameMode)))
  (Variables|Default|SetGameMode_Tutorial _asbp_game_mode_tutorial)
  (bind _asbp_avatar (Utilities|Casting|CastToBP_Avatar (Game|Player|GetPlayerPawn 0)))
  (Variables|Default|SetSpheroid _asbp_avatar)
  (bind _asbp_pickup_key (Utilities|Casting|CastToBP_Pickup_Key (Variables|/Script/Engine.ChildActorComponent|GetChildActor (Variables|Default|GetBaitKey))))
  (Collision|AssignOnComponentBeginOverlap (Variables|/Script/SpheroidX.PickupBase|GetCollision _asbp_pickup_key) (delegate Custom|OnComponentBeginOverlap_Event_0)))

(event Collision|EventActorBeginOverlap
  (params (OtherActor :type Actor%20Object%20Reference)))

(event EventTick
  (params (DeltaSeconds :type Float%20%28single-precision%29)))

(fn ConstructionScript)